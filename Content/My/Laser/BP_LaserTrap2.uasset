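; BP_LaserTrap2 is a laser trap actor that damages the first-person player on contact.
; Capsule overlap with BP_FirstPersonCharacter spawns a scaled explosion at the Niagara beam's location and adds fixed damage through BP_PlayerState.
; DoPlay and DoStop toggle IsPlay, which Tick polls to hide the beam when true and show it when false.
; The flag affects only visibility, so overlap damage applies in either state.
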(event OnComponentBeginOverlap(Capsule)
  (params (OverlappedComponent :type Primitive%20Component%20Object%20Reference) (OtherActor :type Actor%20Object%20Reference) (OtherComp :type Primitive%20Component%20Object%20Reference) (OtherBodyIndex :type Integer) (bFromSweep :type Boolean) (SweepResult :type Hit%20Result%20Structure%20%28by%20ref%29))
  (bind _asbp_first_person_character (Utilities|Casting|CastToBP_FirstPersonCharacter OtherActor))
  (Effects|SpawnEmitteratLocation "/Game/StarterContent/Particles/P_Explosion.P_Explosion" (Transformation|GetWorldLocation (Variables|Default|GetNiagara)) "0, 0, 0" "3.000000,3.000000,3.000000")
  (bind _asbp_player_state (Utilities|Casting|CastToBP_PlayerState (Variables|/Script/Engine.Pawn|GetPlayerState _asbp_first_person_character)))
  (Default|AddDamage _asbp_player_state 1e+01))

(event EventBeginPlay)

(event Collision|EventActorBeginOverlap
  (params (OtherActor :type Actor%20Object%20Reference)))

(event EventTick
  (params (DeltaSeconds :type Float%20%28single-precision%29))
  (if (Variables|Default|GetIsPlay)
    (Rendering|SetVisibility (Variables|Default|GetNiagara) false false)
    (else
      (Rendering|SetVisibility (Variables|Default|GetNiagara) true false))))

(fn ConstructionScript)

(fn DoPlay
  (Variables|Default|SetIsPlay true))

(fn DoStop
  (Variables|Default|SetIsPlay false))