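; BP_PlayerState tracks the player's HP and gold and handles the game-over state.
; CollectGold, AddDamage and RestoreHP update the totals and broadcast them through event dispatchers, passing a hard-coded max HP without clamping.
; Tick polls HP; at zero or below it waits briefly, pauses the game, shows the UW_Died widget and enables the mouse cursor.
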(event EventTick
  (params (DeltaSeconds :type Float%20%28single-precision%29))
  (if (<= (Variables|Default|GetCurrentHP) 0.0)
    (Utilities|FlowControl|Delay 0.5)
    (Game|SetGamePaused true)
    (bind _returnvalue (UserInterface|CreateWidget "/Game/My/위젯/UW_Died.UW_Died_C"))
    (UserInterface|Viewport|AddtoViewport _returnvalue 0)
    (Variables|/Script/Engine.PlayerController|SetbShowMouseCursor (Game|GetPlayerController 0) true)))

(fn ConstructionScript)

(fn CollectGold
  (params (PickUpGold :type Float%20%28double-precision%29))
  (bind _output_get (Variables|Default|SetTotalGold (+ PickUpGold (Variables|Default|GetTotalGold))))
  (Default|CallEventDispatcherCollectGold _output_get))

(fn AddDamage
  (params (B :type Float%20%28double-precision%29))
  (bind _output_get (Variables|Default|SetCurrentHP (- (Variables|Default|GetCurrentHP) B)))
  (Default|CallEventDispatcherChangeHP _output_get 1e+01))

(fn RestoreHP
  (params (Restore :type Float%20%28double-precision%29))
  (bind _output_get (Variables|Default|SetCurrentHP (+ (Variables|Default|GetCurrentHP) Restore)))
  (Default|CallEventDispatcherChangeHP _output_get 1e+01))