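; Moving rectangle Blueprint meant to slide its Cube along local X, with DoPlay and DoStop toggling the motion.
; While enabled, Tick switches on a direction state and nudges the Cube by a fixed per-frame step, not scaled by delta time.
; The Move Left case adds X up to a limit and sets MoveType to MoveRight.
; The Move Right case never moves, as its condition is constant and its lower-bound check is unconnected.
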(event EventTick
  (params (DeltaSeconds :type Float%20%28single-precision%29))
  (if (Variables|Default|GetIsMove)
    (switch Utilities|FlowControl|Switch|SwitchonEN_MoveType "NewEnumerator0"
      (:NewEnumerator0
        (if (not (> (.x (Variables|/Script/Engine.SceneComponent|GetRelativeLocation (Variables|Default|GetCube))) 1.5e+02))
          (Transformation|AddRelativeLocation (Variables|Default|GetCube) (Math|Vector|MakeVector 1.5 0.0 0.0) false false)
          (Variables|Default|SetMoveType "NewEnumerator1")))
      (:NewEnumerator1
        (if (not true)
          (Transformation|AddRelativeLocation (Variables|Default|GetCube) (Math|Vector|MakeVector -1.5 0.0 0.0) false false))))))

(fn ConstructionScript)

(fn DoStop
  (Variables|Default|SetIsMove false))

(fn DoPlay
  (Variables|Default|SetIsMove true))