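; BP_MoveRectFloor is a moving floor Blueprint that slides its Cube component back and forth along its local X axis.
; Each Tick, the MoveType state selects the direction, adds a fixed relative offset and flips the state when the cube passes either end of its range.
; The step is not scaled by delta time, so movement speed depends on frame rate.
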(event EventTick
  (params (DeltaSeconds :type Float%20%28single-precision%29))
  (switch Utilities|FlowControl|Switch|SwitchonEN_MoveType (Variables|Default|GetMoveType)
    (:NewEnumerator0
      (Transformation|AddRelativeLocation (Variables|Default|GetCube) (Math|Vector|MakeVector 1.5 0.0 0.0) false false)
      (if (> (.x (Variables|/Script/Engine.SceneComponent|GetRelativeLocation (Variables|Default|GetCube))) 1.5e+02)
        (Variables|Default|SetMoveType "NewEnumerator1")))
    (:NewEnumerator1
      (Transformation|AddRelativeLocation (Variables|Default|GetCube) (Math|Vector|MakeVector -1.5 0.0 0.0) false false)
      (if (< (.x (Variables|/Script/Engine.SceneComponent|GetRelativeLocation (Variables|Default|GetCube))) 0.0)
        (Variables|Default|SetMoveType "NewEnumerator0")))))

(fn ConstructionScript)