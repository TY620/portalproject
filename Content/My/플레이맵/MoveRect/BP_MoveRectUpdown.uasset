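; Moving block actor that shifts its Cube component along local Z by a fixed step every Tick, unscaled by delta time.
; IsLeft selects up or down: descent flips upward below -50, while ascent flips downward whenever Z is below 0.
; As written, it rises indefinitely from zero or above, or jitters near -50 after descending.
; DoPlay and DoStop only set the direction to up or down; neither halts movement.
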(event EventTick
  (params (DeltaSeconds :type Float%20%28single-precision%29))
  (if (Variables|Default|GetIsLeft)
    (Transformation|AddRelativeLocation (Variables|Default|GetCube) (Math|Vector|MakeVector 0.0 0.0 1.5) false false)
    (if (> 0.0 (.z (Variables|/Script/Engine.SceneComponent|GetRelativeLocation (Variables|Default|GetCube))))
      (Variables|Default|SetIsLeft false))
    (else
      (Transformation|AddRelativeLocation (Variables|Default|GetCube) (Math|Vector|MakeVector 0.0 0.0 -1.5) false false)
      (if (< (.z (Variables|/Script/Engine.SceneComponent|GetRelativeLocation (Variables|Default|GetCube))) -5e+01)
        (Variables|Default|SetIsLeft true)))))

(fn ConstructionScript)

(fn DoStop
  (Variables|Default|SetIsLeft false))

(fn DoPlay
  (Variables|Default|SetIsLeft true))