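; BP_LaserTrap is a laser trap actor that, as shown, only calculates where its beam would end.
; On BeginPlay it disables Box collision and line traces forward from LaserStart on the Visibility channel, storing the hit point or maximum range in BeamEndPoint.
; CreateBeam spawns the P_Laser emitter at a start location but ignores its end location and is never called here.
; SkillTriggerBox and the construction script are empty.
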(event EventBeginPlay
  (bind _laserstart (Variables|Default|GetLaserStart))
  (Collision|SetCollisionEnabled (Variables|Default|GetBox) "NoCollision")
  (bind _output_get (Variables|Default|SetBeamEndPoint (+ (Transformation|GetWorldLocation _laserstart) (* (Math|Vector|GetForwardVector _laserstart) 5e+03))))
  (bind (_outhit _returnvalue) (Collision|LineTraceByChannel (Transformation|GetWorldLocation (Variables|Default|GetLaserStart)) _output_get "TraceTypeQuery1" false 0 "None"))
  (if _returnvalue
    (Variables|Default|SetBeamEndPoint (.Location (Collision|BreakHitResult _outhit)))))

(fn ConstructionScript)

(fn CreateBeam
  (params (StartLocation :type Vector) (EndLocation :type Vector))
  (Effects|SpawnEmitteratLocation "/Game/My/플레이맵/Laser/P_Laser.P_Laser" StartLocation))

(fn SkillTriggerBox)