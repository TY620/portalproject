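; BP_StartHud is a HUD Blueprint for the start level that displays the player's HP.
; On BeginPlay it creates the HUD widget, adds it to the viewport and binds an event to BP_PlayerState's ChangeHP dispatcher.
; UpdateHP forwards current and maximum HP to the widget's SetHP, with the initial call reading CurrentHP from player state and using a hard-coded maximum.
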(event EventBeginPlay
  (bind _returnvalue (UserInterface|CreateWidget "/Game/My/플레이맵/HUDWidget.HUDWidget_C"))
  (bind _output_get (Variables|Default|SetHUDWidget _returnvalue))
  (UserInterface|Viewport|AddtoViewport _output_get 0)
  (bind _asbp_player_state (Utilities|Casting|CastToBP_PlayerState (Game|GetPlayerState 0)))
  (EventDispatchers|BindEventtoEventDispatcherChangeHP _asbp_player_state (EventDispatchers|CreateEvent :!event UpdateHP))
  (CallFunction|UpdateHP (Variables|/Game/My/플레이맵/BP_PlayerState.BP_PlayerState_C|GetCurrentHP _asbp_player_state) 1e+01))

(fn ConstructionScript)

(fn UpdateHP
  (params (CurHP :type Float%20%28double-precision%29) (MaxHP :type Float%20%28double-precision%29))
  (Default|SetHP (Variables|Default|GetHUDWidget) CurHP MaxHP))