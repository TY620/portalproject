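; BP_Door2 is a sliding door actor that rises to open and lowers to close.
; Its EventComponent's play and stop dispatchers set the IsOpen flag, which DoPlay and DoStop functions also set.
; Tick reads the flag and moves the Door component along relative Z until it reaches the open or closed limit, using a fixed per-frame step without delta-time scaling or sweep.
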(event EventDispatcherDoPlay(EventComponent)
  (Variables|Default|SetIsOpen true))

(event EventDispatcherDoStop(EventComponent)
  (Variables|Default|SetIsOpen false))

(event EventTick
  (params (DeltaSeconds :type Float%20%28single-precision%29))
  (if (Variables|Default|GetIsOpen)
    (if (not (>= (.z (Variables|/Script/Engine.SceneComponent|GetRelativeLocation (Variables|Default|GetDoor))) 1e+02))
      (Transformation|AddRelativeLocation (Variables|Default|GetDoor) "0.000000,0.000000,1.500000" false false))
    (elif (not (< (.z (Variables|/Script/Engine.SceneComponent|GetRelativeLocation (Variables|Default|GetDoor))) 0.0))
      (Transformation|AddRelativeLocation (Variables|Default|GetDoor) "0.000000,0.000000,-1.500000" false false))))

(fn ConstructionScript)

(fn DoPlay
  (CallFunction|DoPlay)
  (Variables|Default|SetIsOpen true))

(fn DoStop
  (Variables|Default|SetIsOpen false))