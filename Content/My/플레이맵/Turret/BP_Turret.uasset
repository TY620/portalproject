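; BP_Turret is an enemy turret that fires bullets at the player character when it sees them.
; Its PawnSensing component filters sightings to BP_FirstPersonCharacter and instantly rotates the turret actor to face that pawn.
; After a short delay it spawns a BP_Bullet at the transform of its Arrow component.
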(event OnSeePawn(PawnSensing)
  (params (Pawn :type Pawn%20Object%20Reference))
  (Utilities|Casting|CastToBP_FirstPersonCharacter Pawn)
  (Transformation|SetActorRotation (Components|GetOwner (Variables|Default|GetMainGun)) (Math|Rotator|FindLookatRotation (Transformation|GetActorLocation) (Transformation|GetActorLocation Pawn)))
  (Utilities|FlowControl|Delay 0.3)
  (Game|SpawnActorfromClass "/Game/My/플레이맵/Turret/BP_Bullet.BP_Bullet_C" (Transformation|GetWorldTransform (Variables|Default|GetArrow)) "Undefined" "MultiplyWithRoot" 0 0))

(fn ConstructionScript)